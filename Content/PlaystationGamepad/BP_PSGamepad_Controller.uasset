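; Player controller for a PlayStation gamepad setup that flies a DefaultPawn and prints pressed keys as an input test.
; On BeginPlay it logs registered devices, flags a first-generation DualShock 4 or reports a WiiMote by device-name substring, and caches HUD, widget and pawn.
; Sticks move and look, triggers descend and ascend.
; Shoulder buttons roll via looping timers that cancel out when both are held.
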(event Custom|Roll%20Right%20Start
  ;[0 0 0 1 12] Roll Right
  (if (not (Variables|Rolling|GetRoll%20Left))
    (Class|PlayerController|AddRollInput 1.0)))

(event Custom|Roll%20Left%20Start
  ;[0 0 0 1 12] Roll Left
  (if (not (Variables|Rolling|GetRoll%20Right))
    (Class|PlayerController|AddRollInput -1.0)))

(event EventBeginPlay
  ;[0 0 0 1 12] Detect Controller - Log Registered Devices - Set HUD and UMG variables | Set Default Pawn variable
  (CallFunction|DetectFirstGeneration)
  (CallFunction|LogRegisteredDevices)
  (bind _asbp_psgamepad_hud (Utilities|Casting|CastToBP_PSGamepad_HUD (HUD|GetHUD)))
  (bind _output_get (Variables|Default|SetHUD _asbp_psgamepad_hud))
  (Variables|Default|SetGamepad%20Widget (Variables|/Game/PlaystationGamepad/BP_PSGamepad_HUD.BP_PSGamepad_HUD_C|GetGamepadWidget _output_get))
  (bind _asdefault_pawn (Utilities|Casting|CastToDefaultPawn (Pawn|GetControlledPawn)))
  (Variables|Movement|SetDefault%20Pawn _asdefault_pawn))

(event Input|GamepadEvents|GamepadLeftTriggerAxis
  (params (AxisValue :type Float%20%28single-precision%29))
  (bind _default_pawn (Variables|Movement|GetDefault%20Pawn))
  ;[0 0 0 1 12] Ascend / Descend
  (if (> AxisValue 0.01)
    (Variables|Movement|SetAction%20Value%20Z (* AxisValue -1.0))
    (Utilities|IsValid _default_pawn
      (:Is%20Valid
        (Class|DefaultPawn|MoveUpWorld _default_pawn (Variables|Movement|GetAction%20Value%20Z))))))

(event Input|GamepadEvents|GamepadRightTriggerAxis
  (params (AxisValue :type Float%20%28single-precision%29))
  (bind _default_pawn (Variables|Movement|GetDefault%20Pawn))
  ;[0 0 0 1 12] Ascend / Descend
  (if (> AxisValue 0.01)
    (Variables|Movement|SetAction%20Value%20Z AxisValue)
    (Utilities|IsValid _default_pawn
      (:Is%20Valid
        (Class|DefaultPawn|MoveUpWorld _default_pawn (Variables|Movement|GetAction%20Value%20Z))))))

(event Input|GamepadEvents|GamepadLeftShoulder
  (params (Key :type Key%20Structure :default "None"))
  ;[0 0 0 1 12] Roll Left
  (:Pressed
    (Variables|Rolling|SetRoll%20Left true)
    (bind _returnvalue (Utilities|Time|SetTimerbyEvent (delegate Custom|Roll%20Left%20Start) (Utilities|Time|GetWorldDeltaSeconds) true))
    (Variables|Rolling|SetRoll%20Left%20Timer _returnvalue))
  (:Released
    (Utilities|Time|ClearandInvalidateTimerbyHandle (Variables|Rolling|GetRoll%20Left%20Timer))
    (Variables|Rolling|SetRoll%20Left false)))

(event Input|KeyboardEvents|AnyKey
  (params (Key :type Key%20Structure :default "None"))
  ;[0 0 0 1 12] Test pressed keys
  (:Pressed
    (Development|PrintString (Utilities|String|ToString(Text) (Class|KismetInputLibrary|KeyGetDisplayName Key)) true true "(R=1.000000,G=0.000000,B=0.632289,A=1.000000)")))

(event Input|GamepadEvents|GamepadRightShoulder
  (params (Key :type Key%20Structure :default "None"))
  ;[0 0 0 1 12] Roll Right
  (:Pressed
    (Variables|Rolling|SetRoll%20Right true)
    (bind _returnvalue (Utilities|Time|SetTimerbyEvent (delegate Custom|Roll%20Right%20Start) (Utilities|Time|GetWorldDeltaSeconds) true))
    (Variables|Rolling|SetRoll%20Right%20Timer _returnvalue))
  (:Released
    (Utilities|Time|ClearandInvalidateTimerbyHandle (Variables|Rolling|GetRoll%20Right%20Timer))
    (Variables|Rolling|SetRoll%20Right false)))

(event Input|GamepadEvents|GamepadRight2D
  (params (AxisValue :type Vector :default "0, 0, 0"))
  ;[0 0 0 1 12] Look
  (Class|PlayerController|AddPitchInput (.y AxisValue))
  (Class|PlayerController|AddYawInput (.x AxisValue)))

(event Input|GamepadEvents|GamepadLeft2D
  (params (AxisValue :type Vector :default "0, 0, 0"))
  (bind _default_pawn (Variables|Movement|GetDefault%20Pawn))
  ;[0 0 0 1 12] Move
  (Utilities|IsValid _default_pawn
    (:Is%20Valid
      (Class|DefaultPawn|MoveRight _default_pawn (.x AxisValue))
      (Class|DefaultPawn|MoveForward _default_pawn (.y AxisValue)))))

(fn ConstructionScript)

(fn LogRegisteredDevices
  (for (_array_element _array_index) (Class|RawInputFunctionLibrary|GetRegisteredDevices)
    (Development|PrintString (Utilities|String|Append "Handle : " (Utilities|String|ToString(Integer) (.handle _array_element)) "  
" "VendorID : " (Utilities|String|ToString(Integer) (.vendorid _array_element)) "  
" "ProductID : " (Utilities|String|ToString(Integer) (.productid _array_element)) "  
" "DeviceName : " (.devicename _array_element) "  
" "ArrayIndex : " (Utilities|String|ToString(Integer) _array_index)) true true "(R=0.000000,G=0.660000,B=1.000000,A=1.000000)" 5.0)))

(fn DetectFirstGeneration
  (for _array_element (Class|RawInputFunctionLibrary|GetRegisteredDevices)
    (Utilities|FlowControl|Sequence
      (:then_0
        (if (Utilities|String|Contains (.devicename _array_element) "05C4")
          (Variables|Default|SetbIsFirstGeneration true)
          (Development|PrintString "!!! FIRST GENERATION DUALSHOCK4 !!!" true true "(R=0.000000,G=0.660000,B=1.000000,A=1.000000)" 3e+01)))
      (:then_1
        (if (Utilities|String|Contains (.devicename _array_element) "057E")
          (Development|PrintString "WiiMote Connected" true true "(R=0.000000,G=0.164337,B=1.000000,A=1.000000)" 3e+01))))))